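; BP_Enemy is an enemy pawn that chases the player and ragdolls when its health runs out.
; A sphere overlap with the third-person character starts an AI MoveTo, which re-issues itself only after each successful arrival.
; Any damage lowers health and spawns a pooled Niagara effect at the enemy's location.
; At zero health the mesh switches to physics simulation, with no logic to stop the chase.
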(event OnComponentBeginOverlap(Sphere)
  (params (OverlappedComponent :type Primitive%20Component%20Object%20Reference) (OtherActor :type Actor%20Object%20Reference) (OtherComp :type Primitive%20Component%20Object%20Reference) (OtherBodyIndex :type Integer) (bFromSweep :type Boolean) (SweepResult :type Hit%20Result%20Structure%20%28by%20ref%29))
  (Utilities|Casting|CastToBP_ThirdPersonCharacter OtherActor)
  (CallFunction|ChasePlayer))

(event Custom|Chase%20Player
  (AI|AIMoveTo self "0, 0, 0" (Game|GetPlayerCharacter 0) 1.2e+02 false
    (:OnSuccess
      (CallFunction|ChasePlayer))))

(event Game|Damage|EventAnyDamage
  (params (Damage :type Float%20%28single-precision%29) (DamageType :type Damage%20Type%20Object%20Reference) (InstigatedBy :type Controller%20Object%20Reference) (DamageCauser :type Actor%20Object%20Reference))
  (Variables|Default|Sethealth (- (Variables|Default|Gethealth) Damage))
  (Niagara|SpawnSystematLocation "/Game/NiagaraSystems/MS_Damage.MS_Damage" (Transformation|GetActorLocation) "0, 0, 0" "1.000000,1.000000,1.000000" true true "AutoRelease")
  (if (<= (Variables|Default|Gethealth) 0.0)
    (Physics|SetSimulatePhysics (Variables|Character|GetMesh) true)))

(fn ConstructionScript)